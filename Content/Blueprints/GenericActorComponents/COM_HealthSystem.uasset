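; Generic actor health component that tracks health, applies damage and broadcasts health updates and death.
; Init fills health and caches the owner's skeletal mesh and first material.
; ApplyDamage subtracts health, then tests death by subtracting damage again from the new value.
; Optional non-lethal hit feedback flashes a damage material via looping timer and FlipFlop, blocking further damage until a second timer restores it.
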(event `/Game/Blueprints/Interfaces/BPI_Initalizable.Init`
  (bind _returnvalue (`Actor.GetComponentByClass` (`self.GetOwner`) "/Script/Engine.SkeletalMeshComponent"))
  (set `self.CurrentHealth` (`self.MaxHealth`))
  (`/Engine/EditorBlueprintResources/StandardMacros.IsValid` _returnvalue
    (:`Is Valid`
      (bind _output_get (set `self.OwnerMesh` _returnvalue))
      (set `self.DefaultMeshMaterial` (`PrimitiveComponent.GetMaterial` _output_get 0)))))

(event `DamageMesh`
  (bind _returnvalue (`KismetSystemLibrary.K2_SetTimerDelegate` (delegate `DamageMeshFlash`) 0.1 true))
  (set `self.ChangeDamageMatTimer` _returnvalue)
  (`KismetSystemLibrary.K2_SetTimerDelegate` (delegate `StopMEshDamage`) 2.0)
  (set `self.CanTakeDamage` false))

(event `DamageMeshFlash`
  (`/Engine/EditorBlueprintResources/StandardMacros.FlipFlop`
    (:`A`
      (`PrimitiveComponent.SetMaterial` (`self.OwnerMesh`) 0 "/Game/Blueprints/Character/M_Damage.M_Damage"))
    (:`B`
      (`PrimitiveComponent.SetMaterial` (`self.OwnerMesh`) 0 (`self.DefaultMeshMaterial`)))))

(event `StopMEshDamage`
  (`KismetSystemLibrary.K2_ClearAndInvalidateTimerHandle` (`self.ChangeDamageMatTimer`))
  (`PrimitiveComponent.SetMaterial` (`self.OwnerMesh`) 0 (`self.DefaultMeshMaterial`))
  (set `self.CanTakeDamage` true))

(fn `ApplyDamage`
  (params (Damage :type Integer))
  (bind _returnvalue (- (`self.CurrentHealth`) Damage))
  (if (`self.CanTakeDamage`)
    (set `self.CurrentHealth` _returnvalue)
    (`self.OnUpdateHealth` (`self.MaxHealth`) (`self.CurrentHealth`))
    (if (< _returnvalue 0)
      (`self.OnCharacterDeath`)
      (elif (`self.CanDamageMesh`)
        (`self.DamageMesh`)))))

(fn `GetHealth`
  (returns (Health :type Integer))
  (return (`self.CurrentHealth`)))