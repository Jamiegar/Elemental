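; Base elemental weapon, filed under staffs, that an interacting character equips to use primary, curve and block abilities.
; Construction registers its COM_Attack components by ability name and assigns them the weapon's Element, warning if none is set.
; On interaction, it snaps to the equip slot of a BPI_ElementalCharacter, then initializes each ability with character, weapon and element.
; Attack events invoke abilities by name, and GetFirePoint returns the character mesh's FirePoint socket location.
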(event `Init`
  (bind _values (`BlueprintMapLibrary.Map_Values` (`self.AbilityComponents`)))
  (for _array_element _values
    (bind _character (message `/Game/Blueprints/Interfaces/BPI_ElementalCharacter.GetCharacter` (`self.EqupitedActor`)))
    (`/Game/Blueprints/ElementalAbilitys/Attacks/COM_Attack.Init` _array_element _character self (`self.Element`))))

(event `/Game/Blueprints/Interfaces/BPI_WeaponAbility.PrimaryAttack`
  (message `/Game/Blueprints/Interfaces/BPI_Abilitys.UseAbility` (`self.GetAbilityByName` "Primary")))

(event `/Game/Blueprints/Interfaces/BPI_WeaponAbility.CurveAttack`
  (message `/Game/Blueprints/Interfaces/BPI_Abilitys.UseAbility` (`self.GetAbilityByName` "Curve")))

(event `/Game/Blueprints/Interfaces/BPI_WeaponAbility.Block`
  (message `/Game/Blueprints/Interfaces/BPI_Abilitys.UseAbility` (`self.GetAbilityByName` "Block")))

(fn `AddAttack`
  (params (AttackName :type String) (AttackCom :type "/Game/Blueprints/ElementalAbilitys/Attacks/COM_Attack Object Reference"))
  (`BlueprintMapLibrary.Map_Add` (`self.AbilityComponents`) AttackName AttackCom))

(fn `GetAbilityByName`
  (params (AbilityName :type String))
  (returns (`Ability Component` :type "/Game/Blueprints/ElementalAbilitys/Attacks/COM_Attack Object Reference"))
  (return (`BlueprintMapLibrary.Map_Find` (`self.AbilityComponents`) AbilityName)))

(fn `GetFirePoint`
  (returns (FirePointPos :type "Vector Structure"))
  (bind _character (message `/Game/Blueprints/Interfaces/BPI_ElementalCharacter.GetCharacter` (`self.EqupitedActor`)))
  (return (`SceneComponent.GetSocketLocation` (`Character.Mesh` _character) "FirePoint")))

(fn `GetWeapon`
  (returns (Weapon :type "/Game/Blueprints/ElementalAbilitys/Staffs/BP_Weapon Object Reference"))
  (return self))

(fn `Interact`
  (params (`Interacting Actor` :type "Actor Object Reference"))
  (returns (Interactable :type "Actor Object Reference"))
  (bind _output_get (set `self.EqupitedActor` `Interacting Actor`))
  (if (`KismetSystemLibrary.DoesImplementInterface` _output_get "/Game/Blueprints/Interfaces/BPI_ElementalCharacter.BPI_ElementalCharacter_C")
    (bind (_equipt_componenet _socket _sockettransform) (message `/Game/Blueprints/Interfaces/BPI_ElementalCharacter.GetEquiptSlot` (`self.EqupitedActor`)))
    (`self.K2_AttachToComponent` _equipt_componenet _socket "SnapToTarget" "SnapToTarget" "SnapToTarget")
    (`SceneComponent.K2_SetWorldTransform` (`self.RootComponent`) _sockettransform false true)
    (`self.Init`)
    (return self)))

(fn `UserConstructionScript`
  (`/Engine/EditorBlueprintResources/StandardMacros.IsValid` (`self.Element`)
    (:`Is Valid`
      (for _array_element (`self.K2_GetComponentsByClass` "/Game/Blueprints/ElementalAbilitys/Attacks/COM_Attack.COM_Attack_C")
        (bind _name (message `/Game/Blueprints/Interfaces/BPI_Abilitys.GetAbilityName` _array_element))
        (`self.AddAttack` _name _array_element)
        (set `/Game/Blueprints/ElementalAbilitys/Attacks/COM_Attack.ElementType` (`self.Element`) _array_element)))
    (:`Is Not Valid`
      (`KismetSystemLibrary.PrintString` "Select Element For Weapon" true true (struct :`R` 1.0 :`B` 0.020756 :`A` 1.0) 5.0))))