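; Fire staff weapon that gives its equipped actor a primary attack and a hold-and-release curved secondary attack, each delegated to an ability component.
; Init binds the actor's primary and secondary inputs.
; Holding secondary locks camera turning and opens a gate, letting Tick bend a Bezier path with mouse X while an enemy target exists.
; Releasing restores the camera, fires the curve attack and closes the gate.
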(event `/Game/Blueprints/Interfaces/BPI_Initalizable.Init`
  (`parent.Init`)
  (add `/Game/Blueprints/Character/BP_ElementalCharacter.InputSecondaryPress` (`self.EqupitedActor`) (`|CreateDelegate` :!event `CurveAttackPress`))
  (add `/Game/Blueprints/Character/BP_ElementalCharacter.InputSecondaryRelease` (`self.EqupitedActor`) (`|CreateDelegate` :!event `CurveAttackRelease`))
  (add `/Game/Blueprints/Character/BP_ElementalCharacter.InputPrimaryPress` (`self.EqupitedActor`) (`|CreateDelegate` :!event `PrimaryAttack`)))

(event `/Game/Blueprints/Interfaces/BPI_WeaponAbility.PrimaryAttack`
  (message `/Game/Blueprints/Interfaces/BPI_Abilitys.UseAbility` (`self.COM_PrimaryAttack`)))

(event `/Game/Blueprints/Interfaces/BPI_WeaponAbility.SecondaryAttack`)

(event `self.ReceiveTick`
  (params (DeltaSeconds :type "Float (single-precision)"))
  (bind _com_curve_attack (`self.COM_Curve_Attack`))
  (`/Engine/EditorBlueprintResources/StandardMacros.IsValid` (`self.EqupitedActor`)
    (:`Is Valid`
      (bind _target (`/Game/Blueprints/ElementalAbilitys/Attacks/COM_Curve_Attack.FindTarget` _com_curve_attack))
      (bind _output_get (set `/Game/Blueprints/ElementalAbilitys/Attacks/COM_Curve_Attack.Enemy Target` _target _com_curve_attack))
      (`/Engine/EditorBlueprintResources/StandardMacros.IsValid` _output_get
        (:`Is Valid`
          (`/Engine/EditorBlueprintResources/StandardMacros.Gate` true :!label _label
            (:`Exit`
              (`/Game/Blueprints/ElementalAbilitys/Attacks/COM_Curve_Attack.SetBezierPositions` (`self.COM_Curve_Attack`) (`/Game/Controllers/C_ElementalController.Get Mouse X Axis` (`/Game/Blueprints/Character/BP_ElementalCharacter.Get Elemental Controller` (`self.EqupitedActor`)))))))))))

(event `CurveAttackPress`
  (set `ElementalPlayerCharacter._cameraCanTurn` false (`self.EqupitedActor`))
  (`/Game/Blueprints/ElementalAbilitys/Attacks/COM_Curve_Attack.Set inital Positions` (`self.COM_Curve_Attack`))
  (goto _label :!via `Open`))

(event `CurveAttackRelease`
  (set `ElementalPlayerCharacter._cameraCanTurn` true (`self.EqupitedActor`))
  (message `/Game/Blueprints/Interfaces/BPI_Abilitys.UseAbility` (`self.COM_Curve_Attack`))
  (goto _label :!via `Close`))

(fn `UserConstructionScript`
  (`parent.UserConstructionScript`))