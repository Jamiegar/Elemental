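; BP_Staff is an equippable staff weapon that lets an elemental character perform primary and curve attacks.
; On interact, it attaches to the equip slot socket supplied through BPI_ElementalCharacter and returns itself.
; It gathers its COM_Attack components at construction and initializes each with the character and staff when equipped.
; Attack events delegate to those components, passing an enemy target for curve attacks, and FirePoint socket getters expose location and direction.
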(event `Init`
  (for _array_element (`self.AttackComponents`)
    (bind _character (message `/Game/Blueprints/Interfaces/BPI_ElementalCharacter.GetCharacter` (`self.EqupitedActor`)))
    (`/Game/Blueprints/ElementalAbilitys/Staffs/Attacks/COM_Attack.Init` _array_element _character self)))

(event `/Game/Blueprints/Interfaces/BPI_Weapon.PrimaryAttack`
  (`/Game/Blueprints/ElementalAbilitys/Staffs/Attacks/COM_Attack.UseAttack` (`self.COM_PrimaryAttack`)))

(event `/Game/Blueprints/Interfaces/BPI_Weapon.CurveAttack`
  (params (EnemyTarget :type "Actor Object Reference"))
  (bind _com_curve_attack (`self.COM_Curve_Attack`))
  (set `/Game/Blueprints/ElementalAbilitys/Staffs/Attacks/COM_Curve_Attack.Enemy Target` EnemyTarget _com_curve_attack)
  (`/Game/Blueprints/ElementalAbilitys/Staffs/Attacks/COM_Attack.UseAttack` _com_curve_attack))

(fn `GetFirePoint`
  (returns (FirePointPos :type "Vector Structure"))
  (return (`SceneComponent.GetSocketLocation` (`self.StaticMesh`) "FirePoint")))

(fn `GetFirePointForwardVector`
  (returns (ForwardVector :type "Vector Structure"))
  (return (`KismetMathLibrary.Normal` (`KismetMathLibrary.GetForwardVector` (`SceneComponent.GetSocketRotation` (`self.StaticMesh`) "FirePoint")))))

(fn `Interact`
  (params (`Interacting Actor` :type "Actor Object Reference"))
  (returns (Interactable :type "Actor Object Reference"))
  (bind _output_get (set `self.EqupitedActor` `Interacting Actor`))
  (if (`KismetSystemLibrary.DoesImplementInterface` _output_get "/Game/Blueprints/Interfaces/BPI_ElementalCharacter.BPI_ElementalCharacter_C")
    (bind (_equipt_componenet _socket) (message `/Game/Blueprints/Interfaces/BPI_ElementalCharacter.GetEquiptSlot` (`self.EqupitedActor`)))
    (`self.K2_AttachToComponent` _equipt_componenet _socket "SnapToTarget" "SnapToTarget" "SnapToTarget")
    (`self.Init`)
    (return self)))

(fn `UserConstructionScript`
  (set `self.AttackComponents` (`self.K2_GetComponentsByClass` "/Game/Blueprints/ElementalAbilitys/Staffs/Attacks/COM_Attack.COM_Attack_C")))