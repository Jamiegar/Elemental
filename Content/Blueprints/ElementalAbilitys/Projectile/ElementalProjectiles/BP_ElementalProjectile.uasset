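; Base elemental projectile actor that takes its flight and impact Niagara effects at initialization and starts a lifetime timer.
; Each tick it sphere-traces a short distance ahead of its arrow, ignoring the instigator, with debug drawing on.
; On a hit it sends the result to the hit actor through a message, spawns the impact effect at its own location and destroys itself.
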(event `/Game/Blueprints/Interfaces/BPI_ElementalForceProjectile.InitProjectile`
  (params (`ProjectilHit VFX` :type "NiagaraSystem Object Reference") (`Projectile VFX` :type "NiagaraSystem Object Reference"))
  (set `self.HitVFX` `ProjectilHit VFX`)
  (bind _output_get (set `self.ProjectileVFX` `Projectile VFX`))
  (`NiagaraComponent.SetAsset` (`self.Niagara`) _output_get true)
  (`self.SetActorTickEnabled` true)
  (`KismetSystemLibrary.K2_SetTimerDelegate` (`|CreateDelegate` :!event `DestroyAfterLifeTime`) (`self.LifeTime`)))

(event `self.ReceiveTick`
  (params (DeltaSeconds :type "Float (single-precision)"))
  (`self.CheckForHit`))

(event `CheckForHit`
  (bind _returnvalue (`SceneComponent.K2_GetComponentLocation` (`self.Arrow`)))
  (bind (_outhit _returnvalue_2) (`KismetSystemLibrary.SphereTraceSingle` _returnvalue (+ _returnvalue (* (`SceneComponent.GetForwardVector` (`self.Arrow`)) 5.0)) 5.0 "TraceTypeQuery4" false (`|MakeArray` (`self.GetInstigator`) :!type "Actor Object Reference") "ForDuration" true (struct :`R` 1.0 :`A` 1.0) (struct :`G` 1.0 :`A` 1.0) 0.0))
  (if _returnvalue_2
    (`self.OnProjectileHit` _outhit)
    (`self.SetActorTickEnabled` false)
    (bind (_bblockinghit _binitialoverlap _time _distance _location _impactpoint _normal _impactnormal _physmat _hitactor _hitcomponent _hitbonename) (`GameplayStatics.BreakHitResult` _outhit))
    (`KismetSystemLibrary.PrintString` (`KismetSystemLibrary.GetDisplayName` _hitcomponent))
    (`KismetSystemLibrary.PrintString` (`KismetStringLibrary.Conv_NameToString` _hitbonename))))

(fn `DestroyAfterLifeTime`
  (`self.K2_DestroyActor`))

(fn `OnProjectileHit`
  (params (HitResult :type "HitResult Structure"))
  (message `/Game/Blueprints/Interfaces/BPI_Damageable.OnProjectileActorHit` (`.HitActor` (`GameplayStatics.BreakHitResult` HitResult)) HitResult)
  (`self.SpawnImpactVFX`)
  (`self.K2_DestroyActor`))

(fn `SpawnImpactVFX`
  (`NiagaraFunctionLibrary.SpawnSystemAtLocation` (`self.HitVFX`) (`self.K2_GetActorLocation`)))

(fn `UserConstructionScript`)