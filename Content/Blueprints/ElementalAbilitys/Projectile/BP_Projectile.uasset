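; Elemental ability projectile actor that takes its flight and impact VFX from the element passed to InitProjectile.
; Init sets the Niagara asset, enables tick and starts a lifetime timer.
; Each tick runs a short forward line trace from the Arrow, with debug drawing, rather than using overlap events.
; On a hit it forwards the result to the target's COM_PhysicalAnim, then spawns impact VFX and destroys itself if the element is valid.
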(event `/Game/Blueprints/Interfaces/BPI_ForceProjectile.InitProjectile`
  (params (Element :type "/Game/Blueprints/ElementalAbilitys/DA_ElementalPower Object Reference"))
  (bind _output_get (set `self.ElementalPower` Element))
  (`NiagaraComponent.SetAsset` (`self.Niagara`) (`/Game/Blueprints/ElementalAbilitys/DA_ElementalPower.ProjectileVFX` _output_get) true)
  (`self.SetActorTickEnabled` true)
  (`KismetSystemLibrary.K2_SetTimerDelegate` (`|CreateDelegate` :!event `DestroyAfterLifeTime`) (`self.LifeTime`)))

(event `self.ReceiveTick`
  (params (DeltaSeconds :type "Float (single-precision)"))
  (`self.CheckForHit`))

(event `CheckForHit`
  (bind _returnvalue (`SceneComponent.K2_GetComponentLocation` (`self.Arrow`)))
  (bind (_outhit _returnvalue_2) (`KismetSystemLibrary.LineTraceSingle` :`Start` _returnvalue :`End` (+ _returnvalue (* (`SceneComponent.GetForwardVector` (`self.Arrow`)) 5.0)) :`TraceChannel` "TraceTypeQuery4" :`DrawDebugType` "ForDuration" :`DrawTime` 0.1))
  (if _returnvalue_2
    (`self.OnProjectileHit` _outhit)
    (`self.SetActorTickEnabled` false)
    (bind (_bblockinghit _binitialoverlap _time _distance _location _impactpoint _normal _impactnormal _physmat _hitactor _hitcomponent _hitbonename) (`GameplayStatics.BreakHitResult` _outhit))
    (`KismetSystemLibrary.PrintString` (`KismetSystemLibrary.GetDisplayName` _hitcomponent))
    (`KismetSystemLibrary.PrintString` (`KismetStringLibrary.Conv_NameToString` _hitbonename))))

(event `OnProjectileHit`
  (params (HitResult :type "HitResult Structure"))
  (bind _elementalpower (`self.ElementalPower`))
  (`/Game/Blueprints/Character/COM_PhysicalAnim.Hit` (`self.GetComponentByClass` (`.HitActor` (`GameplayStatics.BreakHitResult` HitResult)) "/Game/Blueprints/Character/COM_PhysicalAnim.COM_PhysicalAnim_C") HitResult)
  (`/Engine/EditorBlueprintResources/StandardMacros.IsValid` _elementalpower
    (:`Is Valid`
      (`NiagaraFunctionLibrary.SpawnSystemAtLocation` (`/Game/Blueprints/ElementalAbilitys/DA_ElementalPower.ProjectileHitVFX` _elementalpower) (`self.K2_GetActorLocation`))
      (`self.K2_DestroyActor`))))

(fn `DestroyAfterLifeTime`
  (`self.K2_DestroyActor`))

(fn `SpawnImpactVFX`
  (`NiagaraFunctionLibrary.SpawnSystemAtLocation` (`/Game/Blueprints/ElementalAbilitys/DA_ElementalPower.ProjectileHitVFX` (`self.ElementalPower`))))

(fn `UserConstructionScript`)