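; Elemental staff weapon that characters pick up, with mesh, effects and two abilities supplied by its Element asset.
; Interact snaps it to the character's equip slot, then adds the ability components, maps them by name and binds their input.
; Dropping disables ability ticking and unbinds input.
; It also tracks a mana pool shown on the player UI, supplies the FirePoint socket location and can build spline-mesh projectile paths.
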(event `/Game/Blueprints/Interfaces/BPI_Initalizable.Init`
  (`|AddComponentByClass` (`/Game/Blueprints/ElementalAbilitys/DA_ElementalPower.PrimaryAbility` (`self.Element`)))
  (`|AddComponentByClass` (`/Game/Blueprints/ElementalAbilitys/DA_ElementalPower.SecondaryAbility` (`self.Element`)))
  (`self.FindAttachedAbilitys`)
  (`/Game/Blueprints/UI/UI_Game.SetUIElement` (`/Game/Blueprints/Character/BP_ElementalCharacterWizzard.PlayerUI` (`self.EqupitedActor`)) (`self.Element`))
  (bind _values (`BlueprintMapLibrary.Map_Values` (`self.AbilityComponents`)))
  (for _array_element _values
    (bind _character (message `/Game/Blueprints/Interfaces/BPI_ElementalCharacter.GetCharacter` (`self.EqupitedActor`)))
    (`/Engine/EditorBlueprintResources/StandardMacros.IsValid` _character
      (:`Is Valid`
        (`/Game/Blueprints/ElementalAbilitys/Attacks/COM_Attack.Init Ability` _array_element _character self (`self.Element`))
        (message `/Game/Blueprints/Interfaces/BPI_Abilitys.BindAbilityInputActions` _array_element (`self.EqupitedActor`))
        (`KismetSystemLibrary.PrintString` (`KismetStringLibrary.Concat_StrStr` "Initalized Ability: " (`KismetSystemLibrary.GetDisplayName` _array_element)) true true (struct :`G` 0.984682 :`B` 1.0 :`A` 1.0) 5.0))
      (:`Is Not Valid`
        (`KismetSystemLibrary.PrintString` "Ability Initalization Failed: Equipted Actor == NULL" true true (struct :`R` 1.0 :`B` 0.047235 :`A` 1.0))))))

(event `self.OnPickUp`
  (`/Game/Blueprints/Interfaces/BPI_Initalizable.Init`)
  (`/Game/SFXData/BPFL_Sound.PlaySound` self (`/Game/Blueprints/ElementalAbilitys/DA_ElementalPower.PickUpSFX` (`self.Element`)) (`self.K2_GetActorLocation`))
  (`NiagaraFunctionLibrary.SpawnSystemAtLocation` (`/Game/Blueprints/ElementalAbilitys/DA_ElementalPower.PickUpVFX` (`self.Element`)) (`SceneComponent.K2_GetComponentLocation` (`/Game/Blueprints/Character/BP_ElementalCharacterWizzard.FeetPosition` (`self.EqupitedActor`))))
  (bind _values (`BlueprintMapLibrary.Map_Values` (`self.AbilityComponents`)))
  (for _array_element _values
    (`ActorComponent.SetComponentTickEnabled` _array_element true)))

(event `self.OnDrop`
  (`PrimitiveComponent.SetCollisionEnabled` (`self.Capsule`) "QueryOnly")
  (bind _values (`BlueprintMapLibrary.Map_Values` (`self.AbilityComponents`)))
  (for _array_element _values
    (`ActorComponent.SetComponentTickEnabled` _array_element false)
    (message `/Game/Blueprints/Interfaces/BPI_Abilitys.UnBindAbilityInputActions` _array_element (`self.EqupitedActor`)))
  (set `self.EqupitedActor` null))

(fn `AddAttack`
  (params (AttackName :type String) (AttackCom :type "/Game/Blueprints/ElementalAbilitys/Attacks/COM_Attack Object Reference"))
  (if (not (`BlueprintMapLibrary.Map_Contains` (`self.AbilityComponents`) (`local.AttackName`)))
    (`BlueprintMapLibrary.Map_Add` (`self.AbilityComponents`) (`local.AttackName`) (`local.AttackCom`))))

(fn `AddMana`
  (params (AddingMana :type "Float (double-precision)"))
  (bind _returnvalue (+ AddingMana (`self.CurrentMana`)))
  (if (< _returnvalue (`self.TotalWeaponMana`))
    (set `self.CurrentMana` _returnvalue)
    (`/Game/Blueprints/UI/UI_Game.SetCurrentMana` (`/Game/Blueprints/Character/BP_ElementalCharacterWizzard.PlayerUI` (`self.EqupitedActor`)) (/ _returnvalue (`self.TotalWeaponMana`)))))

(fn `AddProjectilePath`
  (params (ProjectilePath :type "Array of Vector Structure"))
  (for _array_element ProjectilePath
    (`SplineComponent.AddSplinePoint` (`self.Spline`) _array_element "World" true))
  (for _index (range (`SplineComponent.GetNumberOfSplinePoints` (`self.Spline`)))
    (bind _returnvalue (`AddComponent|NODE_AddSplineMeshComponent-1` :`bManualAttachment` true))
    (`KismetArrayLibrary.Array_Add` (`self.SplineMeshes`) _returnvalue)
    (bind (_location _tangent) (`SplineComponent.GetLocationAndTangentAtSplinePoint` (`self.Spline`) _index "World"))
    (bind (_location_2 _tangent_2) (`SplineComponent.GetLocationAndTangentAtSplinePoint` (`self.Spline`) (+ _index 1) "World"))
    (`SplineMeshComponent.SetStartAndEnd` _returnvalue _location _tangent _location_2 _tangent_2 true)))

(fn `ClearSplinePoints`
  (bind _splinemeshes (`self.SplineMeshes`))
  (`SplineComponent.ClearSplinePoints` (`self.Spline`) true)
  (`ActorComponent.K2_DestroyComponent` _splinemeshes)
  (`KismetArrayLibrary.Array_Clear` _splinemeshes))

(fn `FindAttachedAbilitys`
  (bind _returnvalue (`self.K2_GetComponentsByClass` "/Game/Blueprints/ElementalAbilitys/Attacks/COM_Attack.COM_Attack_C"))
  (`/Engine/EditorBlueprintResources/StandardMacros.IsValid` (`self.Element`)
    (:`Is Valid`
      (if (`KismetArrayLibrary.Array_IsValidIndex` _returnvalue)
        (for _array_element _returnvalue
          (bind _abilitycomponent (message `/Game/Blueprints/Interfaces/BPI_Abilitys.GetAbilityComponent` _array_element))
          (bind _name (message `/Game/Blueprints/Interfaces/BPI_Abilitys.GetAbilityName` _abilitycomponent))
          (if (`KismetStringLibrary.IsEmpty` _name)
            (`KismetSystemLibrary.PrintString` (`KismetStringLibrary.Concat_StrStr` (`KismetSystemLibrary.GetDisplayName` _abilitycomponent) ": has no ability name") true true (struct :`R` 1.0 :`B` 0.018806 :`A` 1.0) 5.0)
            (else
              (`self.AddAttack` _name _abilitycomponent)
              (set `/Game/Blueprints/ElementalAbilitys/Attacks/COM_Attack.ElementType` (`self.Element`) _abilitycomponent))))
        (else
          (`KismetSystemLibrary.PrintString` "No Attached Abilitys" true true (struct :`R` 1.0 :`G` 0.015401 :`A` 1.0)))))
    (:`Is Not Valid`
      (`KismetSystemLibrary.PrintString` "Select Element For Weapon" true true (struct :`R` 1.0 :`B` 0.020756 :`A` 1.0) 5.0))))

(fn `GetAbilityByName`
  (params (AbilityName :type String))
  (returns (`Ability Component` :type "/Game/Blueprints/ElementalAbilitys/Attacks/COM_Attack Object Reference"))
  (return (`BlueprintMapLibrary.Map_Find` (`self.AbilityComponents`) AbilityName)))

(fn `GetFirePoint`
  (returns (FirePointPos :type "Vector Structure"))
  (bind _character (message `/Game/Blueprints/Interfaces/BPI_ElementalCharacter.GetCharacter` (`self.EqupitedActor`)))
  (`/Engine/EditorBlueprintResources/StandardMacros.IsValid` _character
    (:`Is Valid`
      (return (`SceneComponent.GetSocketLocation` (`Character.Mesh` _character) "FirePoint")))))

(fn `GetManaCostForAbility`
  (params (AbilityManaCost :type "Float (double-precision)"))
  (returns (CanUseAbility :type Boolean))
  (if (>= (- (`self.CurrentMana`) AbilityManaCost) 0.0)
    (return true)
    (else
      (return false))))

(fn `GetWeapon`
  (returns (Weapon :type "/Game/Blueprints/ElementalAbilitys/BP_Weapon Object Reference"))
  (return self))

(fn `Interact`
  (params (`Interacting Actor` :type "Actor Object Reference"))
  (returns (Interactable :type "Actor Object Reference"))
  (bind _character (message `/Game/Blueprints/Interfaces/BPI_ElementalCharacter.GetCharacter` `Interacting Actor`))
  (bind _output_get (set `self.EqupitedActor` _character))
  (`/Engine/EditorBlueprintResources/StandardMacros.IsValid` _output_get
    (:`Is Valid`
      (bind (_equipt_componenet _socket _sockettransform) (message `/Game/Blueprints/Interfaces/BPI_ElementalCharacter.GetEquiptSlot` (`self.EqupitedActor`)))
      (`self.K2_AttachToComponent` _equipt_componenet _socket "SnapToTarget" "SnapToTarget" "SnapToTarget")
      (`SceneComponent.K2_SetWorldTransform` (`self.RootComponent`) _sockettransform false true)
      (`self.OnPickUp`)
      (`PrimitiveComponent.SetCollisionEnabled` (`self.Capsule`) "NoCollision")
      (return self))
    (:`Is Not Valid`
      (`KismetSystemLibrary.PrintString` "Interaction Unseccessful: Interacting character == NULL"))))

(fn `OnWeaponAbilityUsed`
  (params (AbilityManaCost :type "Float (double-precision)"))
  (if (`self.GetManaCostForAbility` AbilityManaCost)
    (bind _output_get (set `self.CurrentMana` (- (`self.CurrentMana`) (`local.AbilityManaCost`))))
    (`/Game/Blueprints/UI/UI_Game.SetCurrentMana` (`/Game/Blueprints/Character/BP_ElementalCharacterWizzard.PlayerUI` (`self.EqupitedActor`)) (/ _output_get (`self.TotalWeaponMana`)))
    (`PlayerCameraManager.StartCameraShake` :`self` (`GameplayStatics.GetPlayerCameraManager` 0) :`ShakeClass` "/Game/Blueprints/Env/CameraShake/BP_PlayerAbilityUse_Shake.BP_PlayerAbilityUse_Shake_C")))

(fn `UserConstructionScript`
  (`/Engine/EditorBlueprintResources/StandardMacros.IsValid` (`self.Element`)
    (:`Is Valid`
      (`StaticMeshComponent.SetStaticMesh` (`self.StaticMesh`) (`/Game/Blueprints/ElementalAbilitys/DA_ElementalPower.StaffMesh` (`self.Element`)))
      (set `self.CurrentMana` (`self.TotalWeaponMana`)))
    (:`Is Not Valid`
      (`KismetSystemLibrary.PrintString` "Select Element For Weapon" true true (struct :`R` 1.0 :`B` 0.020756 :`A` 1.0) 5.0))))