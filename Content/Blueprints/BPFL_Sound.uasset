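; BPFL_Sound is a sound helper library that plays a given SFX on behalf of an instigator.
; PlaySound switches on the SFX's SoundType, playing 2D sounds without position and 3D sounds at the supplied location.
; Both branches get the cue from the SFX's GetSoundCue and use the instigator as world context.
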(fn `PlaySound`
  (params (Instogator :type "Actor Object Reference") (SFX :type "/Game/SFXData/DA_SoundData Object Reference") (Location :type "Vector Structure"))
  (switch `/Game/SFXData/Enum_SoundType` (`/Game/SFXData/DA_SoundData.SoundType` SFX)
    (:`NewEnumerator0`
      (`GameplayStatics.PlaySound2D` (`local.Instogator`) (`/Game/SFXData/DA_SoundData.GetSoundCue` (`local.SFX`)) 1.0 1.0 0.0 null null))
    (:`NewEnumerator1`
      (`GameplayStatics.PlaySoundAtLocation` (`local.Instogator`) (`/Game/SFXData/DA_SoundData.GetSoundCue` (`local.SFX`)) (`local.Location`) (struct) 1.0 1.0 0.0 null null null null))))