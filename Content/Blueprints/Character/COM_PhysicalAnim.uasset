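; Actor component that gives its owning character physics-driven hit reactions through a Physical Animation component added to the owner's skeletal mesh on Init.
; Hit applies the StrengthHit profile, simulates bodies below the pelvis, adds a trace-axis impulse at the hit bone (spine_01 for pelvis hits) and extends a timer.
; Tick fades physics blend weight with that timer, then stops simulation and its own ticking.
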(event `/Game/Blueprints/Interfaces/BPI_Initalizable.Init`
  (bind _returnvalue (`Actor.GetComponentByClass` (`self.GetOwner`) "/Script/Engine.SkeletalMeshComponent"))
  (bind _returnvalue_2 (`|AddComponentByClass` (`self.GetOwner`) "/Script/Engine.PhysicalAnimationComponent"))
  (bind _output_get (set `self.PhysicalAnimationComp` _returnvalue_2))
  (`PhysicalAnimationComponent.SetSkeletalMeshComponent` _output_get _returnvalue)
  (set `self.SkeletalMesh` _returnvalue))

(event `TogglePhysicalAnim`
  (`SkeletalMeshComponent.SetAllBodiesBelowSimulatePhysics` (`self.SkeletalMesh`) "Pelvis" true false)
  (`SkeletalMeshComponent.SetAllBodiesBelowPhysicsBlendWeight` (`self.SkeletalMesh`) "Pelvis" 0.5 false true))

(event `self.ReceiveTick`
  (params (DeltaSeconds :type "Float (single-precision)"))
  (bind _output_get (set `self.HitReactionTimeRemaining` (- (`KismetMathLibrary.FInterpTo` (`self.HitReactionTimeRemaining`) 0.0 DeltaSeconds 0.8) (* DeltaSeconds 0.1))))
  (if (<= _output_get 0.0)
    (set `self.HitReactionTimeRemaining` 0.0)
    (`SkeletalMeshComponent.SetAllBodiesBelowSimulatePhysics` (`self.SkeletalMesh`) "Pelvis" false false)
    (`self.SetComponentTickEnabled` false)
    (else
      (`SkeletalMeshComponent.SetAllBodiesBelowPhysicsBlendWeight` (`self.SkeletalMesh`) "Pelvis" (`KismetMathLibrary.FMin` (`self.HitReactionTimeRemaining`) 1.0) false true))))

(event `Hit`
  (params (Hit :type "HitResult Structure"))
  (bind (_bblockinghit _binitialoverlap _time _distance _location _impactpoint _normal _impactnormal _physmat _hitactor _hitcomponent _hitbonename _bonename _hititem _elementindex _faceindex _tracestart _traceend) (`GameplayStatics.BreakHitResult` Hit))
  (`self.SetComponentTickEnabled` true)
  (set `self.HitReactionTimeRemaining` (+ (`self.HitReactionTimeRemaining`) 1.0))
  (`PhysicalAnimationComponent.ApplyPhysicalAnimationProfileBelow` (`self.PhysicalAnimationComp`) "Pelvis" "StrengthHit" false false)
  (`SkeletalMeshComponent.SetAllBodiesBelowSimulatePhysics` (`self.SkeletalMesh`) "Pelvis" true false)
  (`PrimitiveComponent.AddImpulse` (`self.SkeletalMesh`) (* (`KismetMathLibrary.Normal` (- _tracestart _traceend)) 5000.0) (select `bool` (== _bonename "Pelvis") :`false` _bonename :`true` "spine_01") false))