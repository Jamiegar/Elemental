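; Game mode manager that handles timed mana orb spawning at spawn points placed in the level.
; Init starts a looping timer on the configured spawn interval, and StopManaSpawning clears it through the stored handle.
; Helper functions cache every BP_ManaSpawnPoint actor in the level and spawn a scaled-down BP_ManaOrb at each cached location.
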(event `/Game/Blueprints/Interfaces/BPI_Initalizable.Init`
  (bind _returnvalue (`KismetSystemLibrary.K2_SetTimerDelegate` (`|CreateDelegate` :!event `SpawnOrbAtEachLocation`) (`self.TimeBetweenManaSpawn`) true))
  (set `self.ManaSpawnHandle` _returnvalue))

(event `StopManaSpawning`
  (`KismetSystemLibrary.K2_ClearAndInvalidateTimerHandle` (`self.ManaSpawnHandle`)))

(fn `GetAllManaSpawnPointsInLevel`
  (bind _outactors (`GameplayStatics.GetAllActorsOfClass` "/Game/Blueprints/Env/Mana/BP_ManaSpawnPoint.BP_ManaSpawnPoint_C"))
  (set `self.ManaSpawnPoints` _outactors))

(fn `SpawnOrbAtEachLocation`
  (for _array_element (`self.ManaSpawnPoints`)
    (`|SpawnActorFromClass` "/Game/Blueprints/Env/Mana/BP_ManaOrb.BP_ManaOrb_C" (`KismetMathLibrary.MakeTransform` (`self.K2_GetActorLocation` _array_element) (struct) (0.1 0.1 0.1)) "Undefined" "OverrideRootScale" null null)))

(fn `UserConstructionScript`)