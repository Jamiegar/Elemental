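; Player manager that spawns the wizard character at the PlayerStart, possesses it, and manages its input, UI and gate flow.
; Game state changes toggle HUD and movement, switching to UI-only input with cursor after the boss fight.
; Player interaction activates the gate; its permanent closing deactivates it and starts the AI cinematic state.
; The death animation's end requests a scene restart and shows an animated death screen.
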(event `/Game/Blueprints/Interfaces/BPI_Initalizable.Init`
  (`self.CreateController`)
  (`self.Create Elemental Player`)
  (bind _gamestate (message `/Game/Blueprints/Interfaces/BPI_GameState.GetElementalGameState` (`GameplayStatics.GetGameState`)))
  (add `/Game/Blueprints/GameMode/BP_Gamestate.OnGameStateChange` _gamestate (`|CreateDelegate` :!event `OnStateChange`))
  (add `/Game/Blueprints/Inventory/COM_PlayerInventory.OnPlayerInteract` (`/Game/Blueprints/Character/BP_ElementalCharacterWizzard.COM_PlayerInventory` (`self.ElementalPlayer`)) (`|CreateDelegate` :!event `OnPlayerInteracted`))
  (add `/Game/Blueprints/Env/BP_Gate.OnGateClosedPermanently` (`self.Gate`) (`|CreateDelegate` :!event `OnPlayerEnteredThroughGate`))
  (add `/Game/Blueprints/Character/Animation/AnimBP_Elemental.OnAnimationDeathFinished` (`/Game/Blueprints/Character/BP_ElementalCharacterWizzard.GetAnimationInstance` (`self.ElementalPlayer`)) (`|CreateDelegate` :!event `OnCharacterDeath`)))

(event `OnStateChange`
  (params (`New Game State` :type "/Game/Blueprints/GameMode/Enum_GameModeStates Enum" :default "NewEnumerator8"))
  (switch `/Game/Blueprints/GameMode/Enum_GameModeStates` `New Game State`
    (:`NewEnumerator10`
      (`self.SetPlayerUIHidden`))
    (:`NewEnumerator14`
      (`self.SetPlayerUIVisable`))
    (:`NewEnumerator12`
      (`self.SetPlayerUIHidden`)
      (`WidgetBlueprintLibrary.SetInputMode_UIOnlyEx` (`self.PlayerController`) null)
      (set `PlayerController.bShowMouseCursor` true (`self.PlayerController`)))))

(event `SetPlayerUIHidden`
  ;[1 1 1] Player Ui Visability
  (`Widget.SetVisibility` (`/Game/Blueprints/Character/BP_ElementalCharacterWizzard.PlayerUI` (`self.ElementalPlayer`)) "Hidden")
  (set `ElementalCharacter._canMove` false (`self.ElementalPlayer`)))

(event `OnPlayerInteracted`
  (set `/Game/Blueprints/Env/BP_Gate.GateActive` true (`self.Gate`)))

(event `SetPlayerUIVisable`
  ;[1 1 1] Player Ui Visability
  (`Widget.SetVisibility` (`/Game/Blueprints/Character/BP_ElementalCharacterWizzard.PlayerUI` (`self.ElementalPlayer`)) "Visible")
  (set `ElementalCharacter._canMove` true (`self.ElementalPlayer`)))

(event `OnPlayerEnteredThroughGate`
  (set `/Game/Blueprints/Env/BP_Gate.GateActive` false (`self.Gate`))
  (message `/Game/Blueprints/Interfaces/BPI_GameState.ChangeState` (`GameplayStatics.GetGameState`) "NewEnumerator10"))

(event `OnCharacterDeath`
  (bind _gamemode (message `/Game/Blueprints/Interfaces/BPI_ElementalGameMode.GetGameMode` (`GameplayStatics.GetGameMode`)))
  (`/Game/Blueprints/GameMode/GM_Elemental.RestartScene` _gamemode)
  (bind _returnvalue (`|CreateWidget` "/Game/Blueprints/UI/UI_DeathScreen.UI_DeathScreen_C"))
  (`UserWidget.AddToViewport` _returnvalue 0)
  (`/Game/Blueprints/UI/UI_DeathScreen.StartDeathUIAnimation` _returnvalue))

(fn `Create Elemental Player`
  (bind (_returnvalue_location _returnvalue_rotation) (`KismetMathLibrary.BreakTransform` (`self.GetTransform` (`self.PlayeStart`))))
  (bind _returnvalue (`|SpawnActorFromClass` "/Game/Blueprints/Character/BP_ElementalCharacterWizzard.BP_ElementalCharacterWizzard_C" (`KismetMathLibrary.MakeTransform` _returnvalue_location _returnvalue_rotation) "Undefined" "OverrideRootScale" null null))
  (bind _output_get (set `self.ElementalPlayer` _returnvalue))
  (`/Game/Blueprints/Interfaces/BPI_Initalizable.Init` _output_get)
  (`Controller.Possess` (`self.PlayerController`) (`self.ElementalPlayer`)))

(fn `CreateController`
  (bind _controller (message `/Game/Blueprints/Interfaces/BPI_ElementalController.GetController` (`GameplayStatics.GetPlayerController` 0)))
  (bind _output_get (set `self.PlayerController` _controller))
  (`WidgetBlueprintLibrary.SetInputMode_GameOnly` _output_get)
  (set `PlayerController.bShowMouseCursor` false _output_get))

(fn `FadeOutPlayerUI`
  (`/Game/Blueprints/UI/UI_Game.FadeOutAnimation` (`/Game/Blueprints/Character/BP_ElementalCharacterWizzard.PlayerUI` (`self.ElementalPlayer`))))

(fn `GetLevelActors`
  (bind _returnvalue (`GameplayStatics.GetActorOfClass` "/Script/Engine.PlayerStart"))
  (`/Engine/EditorBlueprintResources/StandardMacros.IsValid` _returnvalue
    (:`Is Valid`
      (set `self.PlayeStart` _returnvalue)
      (bind _returnvalue_2 (`GameplayStatics.GetActorOfClass` "/Game/Blueprints/Env/BP_Gate.BP_Gate_C"))
      (`/Engine/EditorBlueprintResources/StandardMacros.IsValid` _returnvalue_2
        (:`Is Valid`
          (set `self.Gate` _returnvalue_2))))))

(fn `GetPlayerController`
  (returns (Controller :type "/Game/Blueprints/Controllers/C_ElementalController Object Reference"))
  (return (`self.PlayerController`)))

(fn `GetPlayerPawn`
  (returns (Character :type "/Game/Blueprints/Character/BP_ElementalCharacterWizzard Object Reference"))
  (return (`self.ElementalPlayer`)))

(fn `UserConstructionScript`)