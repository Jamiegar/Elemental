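; Game mode manager that links the level's elemental AI boss controller to game state changes.
; Init finds and initializes the C_ElementalAI controller, then binds to boss death and game-state events.
; In Game starts the AI and Start Boss Fight begins boss attacks.
; The boss death handler is empty with its PostBossFight change disconnected, and GetAIInLevel, which sets the boss reference, is not called here.
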(event `/Game/Blueprints/Interfaces/BPI_Initalizable.Init`
  (bind _returnvalue (`GameplayStatics.GetActorOfClass` "/Game/Blueprints/Controllers/C_ElementalAI.C_ElementalAI_C"))
  (bind _output_get (set `self.AIBossController` _returnvalue))
  (`/Game/Blueprints/Controllers/C_ElementalAI.Init` _output_get)
  (add `/Game/Blueprints/GenericActorComponents/COM_HealthSystem.OnCharacterDeath` (`/Game/Blueprints/AI/BP_AIBossEnemy.COM_HealthSystem` (`self.AIBoss`)) (`|CreateDelegate` :!event `OnBossDeath`))
  (bind _gamestate (message `/Game/Blueprints/Interfaces/BPI_GameState.GetElementalGameState` (`GameplayStatics.GetGameState`)))
  (add `/Game/Blueprints/GameMode/BP_Gamestate.OnGameStateChange` _gamestate (`|CreateDelegate` :!event `OnGameStateChanged`)))

(event `OnGameStateChanged`
  (params (`New Game State` :type "/Game/Blueprints/GameMode/Enum_GameModeStates Enum" :default "NewEnumerator8"))
  (switch `/Game/Blueprints/GameMode/Enum_GameModeStates` `New Game State`
    (:`NewEnumerator11`
      (`/Game/Blueprints/Controllers/C_ElementalAI.OnAIStart` (`self.AIBossController`)))
    (:`NewEnumerator14`
      (`/Game/Blueprints/Controllers/C_ElementalAI.BeginBossAttacks` (`self.AIBossController`)))))

(event `OnBossDeath`)

(fn `GetAIInLevel`
  (bind _returnvalue (`GameplayStatics.GetActorOfClass` "/Game/Blueprints/AI/BP_AIBossEnemy.BP_AIBossEnemy_C"))
  (set `self.AIBoss` _returnvalue))

(fn `UserConstructionScript`)