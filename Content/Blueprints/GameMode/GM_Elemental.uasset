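; Game mode for Elemental that runs the boss-fight level flow, from initialization through intro cinematic, battle music and victory screen.
; It listens to game state changes and dispatches each phase to an event, some of which advance the state themselves.
; Initialization finds the placed AI, ability, player and mana spawn managers and initializes them through a shared helper.
; It also handles pause toggling, faded scene restart and return to main menu.
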(event `RestartScene`
  ;[1 1 1] Reload scene with camera fade
  (`PlayerCameraManager.StartCameraFade` :`self` (`GameplayStatics.GetPlayerCameraManager` 0) :`ToAlpha` 1.0 :`Duration` 1.5 :`bHoldWhenFinished` true)
  (`/Game/Blueprints/GameMode/Managers/BP_PlayerManager.FadeOutPlayerUI` (`self.PlayerManager`))
  (`KismetSystemLibrary.K2_SetTimerDelegate` (delegate `AfterFadeDuration`) 4.0))

(event `AfterFadeDuration`
  ;[1 1 1] Reload scene with camera fade
  (`GameplayStatics.OpenLevel` "Scene_MeshedLevel" true "game=Elemental"))

(event `self.ReceiveBeginPlay`
  (bind _gamestate (message `/Game/Blueprints/Interfaces/BPI_GameState.GetElementalGameState` (`GameplayStatics.GetGameState`)))
  (bind _output_get (set `self.ElementalGamestate` _gamestate))
  (add `/Game/Blueprints/GameMode/BP_Gamestate.OnGameStateChange` _output_get (`|CreateDelegate` :!event `OnStateChanged`))
  (message `/Game/Blueprints/Interfaces/BPI_Initalizable.Init` _output_get))

(event `Inititalization`
  (`self.InitializeManager` "/Game/Blueprints/GameMode/Managers/BP_AIAbilityManager.BP_AIAbilityManager_C" (`self.AIAbilityManager`))
  (`self.InitializeManager` "/Game/Blueprints/GameMode/Managers/BP_PlayerManager.BP_PlayerManager_C" (`self.PlayerManager`))
  (`self.InitializeManager` "/Game/Blueprints/GameMode/Managers/BP_AIManager.BP_AIManager_C" (`self.AIManager`))
  (`self.InitializeManager` "/Game/Blueprints/GameMode/Managers/BP_ManaSpawnManager.BP_ManaSpawnManager_C" (`self.ManaSpawnerManager`))
  (message `/Game/Blueprints/Interfaces/BPI_GameState.ChangeState` (`GameplayStatics.GetGameState`) "NewEnumerator11"))

(event `SetUpSceneVisuals`
  ;[1 1 1] Camera Fade and background Noise Set up
  (`PlayerCameraManager.StartCameraFade` :`self` (`GameplayStatics.GetPlayerCameraManager` 0) :`FromAlpha` 1.0 :`Duration` 1.5)
  (bind _returnvalue (`/Game/SFXData/BPFL_Sound.PlaySound` self "/Game/SFXData/DataAssets/Environmental/DA_AmbientNoise.DA_AmbientNoise"))
  (set `self.AmbientNoise` _returnvalue))

(event `In Game`
  (`self.SetUpSceneVisuals`)
  (message `/Game/Blueprints/Interfaces/BPI_GameState.ChangeState` (`GameplayStatics.GetGameState`) "NewEnumerator13"))

(event `PreBossFight`)

(event `Cinematic`
  (bind (_outactor _returnvalue) (`LevelSequencePlayer.CreateLevelSequencePlayer` "/Game/Cinematics/Sequences/BossIntroCinamatic/BossIntroCinamaticMaster.BossIntroCinamaticMaster"))
  (`MovieSceneSequencePlayer.Play` _returnvalue)
  (add `MovieSceneSequencePlayer.OnFinished` _returnvalue (delegate `OnCinematicFinished`)))

(event `OnCinematicFinished`
  (message `/Game/Blueprints/Interfaces/BPI_GameState.ChangeState` (`GameplayStatics.GetGameState`) "NewEnumerator14"))

(event `/Game/Blueprints/Interfaces/BPI_ElementalGameMode.SetGamePause`
  (bind _controller (`/Game/Blueprints/GameMode/Managers/BP_PlayerManager.GetPlayerController` (`self.PlayerManager`)))
  (bind _controller_2 (`/Game/Blueprints/GameMode/Managers/BP_PlayerManager.GetPlayerController` (`self.PlayerManager`)))
  ;[1 1 1] Pause
  (if (`GameplayStatics.IsGamePaused`)
    (`GameplayStatics.SetGamePaused` false)
    (set `PlayerController.bShowMouseCursor` false _controller_2)
    (`WidgetBlueprintLibrary.SetInputMode_GameOnly` _controller_2)
    (`Widget.RemoveFromParent` (`self.PauseMenu`))
    (else
      (`GameplayStatics.SetGamePaused` true)
      (set `PlayerController.bShowMouseCursor` true _controller)
      (`WidgetBlueprintLibrary.SetInputMode_GameAndUIEx` _controller null)
      (`/Engine/EditorBlueprintResources/StandardMacros.IsValid` (`self.PauseMenu`) ; Check if pasue menu is valid
        (:`Is Valid`
          _)
        (:`Is Not Valid`
          (bind _returnvalue (`|CreateWidget` "/Game/Blueprints/MenuUserInterface/UI_PauseMenu.UI_PauseMenu_C")) ; If it is not valid create pause menu widget
          (set `self.PauseMenu` _returnvalue)))
      (`UserWidget.AddToViewport` (`self.PauseMenu`) 0) ; Add widget to screen
    )))

(event `StartBossFight`
  (bind _returnvalue (`/Game/SFXData/BPFL_Sound.PlaySound` self "/Game/SFXData/DataAssets/Music/DA_BattleMusic.DA_BattleMusic" (0.0 0.0 0.0)))
  (bind _output_get (set `self.BattleBossMusic` _returnvalue))
  (`AudioComponent.FadeIn` _output_get 3.5 1.0 0.0 "Linear"))

(event `PostBossFight`
  (`PlayerCameraManager.StartCameraFade` :`self` (`GameplayStatics.GetPlayerCameraManager` 0) :`FromAlpha` 0.0 :`ToAlpha` 1.0 :`Duration` 1.5 :`bHoldWhenFinished` true)
  (`AudioComponent.FadeOut` (`self.BattleBossMusic`) 1.5 0.0 "Linear")
  (bind _returnvalue (`|CreateWidget` "/Game/Blueprints/UI/UI_VictoryScreen.UI_VictoryScreen_C"))
  (`UserWidget.AddToViewport` _returnvalue 0)
  (`/Game/Blueprints/UI/UI_VictoryScreen.StartVictoryAnimation` _returnvalue))

(event `/Game/Blueprints/Interfaces/BPI_ElementalGameMode.ReturnToMainMenu`
  (`PlayerCameraManager.StartCameraFade` :`self` (`GameplayStatics.GetPlayerCameraManager` 0) :`ToAlpha` 1.0 :`Duration` 1.5 :`bHoldWhenFinished` true)
  (for _array_element (`|MakeArray` (`self.BattleBossMusic`) (`self.AmbientNoise`))
    (`/Engine/EditorBlueprintResources/StandardMacros.IsValid` _array_element
      (:`Is Valid`
        (`AudioComponent.FadeOut` _array_element 1.5 0.0 "Linear")
        (`/Game/Blueprints/GameMode/Managers/BP_PlayerManager.FadeOutPlayerUI` (`self.PlayerManager`))
        (`KismetSystemLibrary.K2_SetTimerDelegate` (delegate `OnFadeOutsFinished`) 2.0)))))

(event `OnFadeOutsFinished`
  (`GameplayStatics.OpenLevel` "Scene_MainMenu"))

(fn `GetGameMode`
  (returns (GameMode :type "/Game/Blueprints/GameMode/GM_Elemental Object Reference"))
  (return self))

(fn `InitializeManager`
  (params (`Manager Class` :type "Manager Class Reference") (`Manager Variable` :type "Manager Object Reference (by ref)"))
  (bind _returnvalue (`GameplayStatics.GetActorOfClass` `Manager Class`))
  (`/Engine/EditorBlueprintResources/StandardMacros.IsValid` _returnvalue
    (:`Is Valid`
      (`|VariableSetRef` `Manager Variable` _returnvalue)
      (message `/Game/Blueprints/Interfaces/BPI_Initalizable.Init` _returnvalue)
      (`KismetArrayLibrary.Array_Add` (`self.Managers`) _returnvalue))))

(fn `OnStateChanged`
  (params (GameState :type "/Game/Blueprints/GameMode/Enum_GameModeStates Enum" :default "NewEnumerator0"))
  (switch `/Game/Blueprints/GameMode/Enum_GameModeStates` GameState
    (:`NewEnumerator8`
      (`self.Inititalization`))
    (:`NewEnumerator11`
      (`self.In Game`))
    (:`NewEnumerator13`
      (`self.PreBossFight`))
    (:`NewEnumerator10`
      (`self.Cinematic`))
    (:`NewEnumerator14`
      (`self.StartBossFight`))
    (:`NewEnumerator12`
      (`self.PostBossFight`))))

(fn `UserConstructionScript`)