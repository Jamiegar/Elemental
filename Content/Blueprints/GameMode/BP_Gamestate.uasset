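; Game state Blueprint that tracks the match phase of an elemental, staff-based game, from initialization through pre-game, AI cinematic, in-game and post-game.
; ChangeState calls ChangeGameState, which stores the new phase, runs that phase's handler, then fires OnGameStateChange for other systems.
; Init broadcasts the current state, and GetElementalGameState returns self.
; Phase handlers are placeholders that only print debug messages or are empty.
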(event `/Game/Blueprints/Interfaces/BPI_Initalizable.Init`
  (`self.OnGameStateChange` (`self.GameState`)))

(event `/Game/Blueprints/Interfaces/BPI_GameState.ChangeState`
  (params (NewState :type "/Game/Blueprints/GameMode/Enum_GameModeStates Enum" :default "NewEnumerator8"))
  (`self.ChangeGameState` NewState))

(fn `AICinematic`
  (`KismetSystemLibrary.PrintString` "AI Cinematic"))

(fn `ChangeGameState`
  (params (GameState :type "/Game/Blueprints/GameMode/Enum_GameModeStates Enum" :default "NewEnumerator0"))
  (bind _gamestate (`local.GameState`))
  (bind _output_get (set `self.GameState` GameState))
  (switch `/Game/Blueprints/GameMode/Enum_GameModeStates` _output_get
    (:`NewEnumerator8`
      (`self.Initialization`))
    (:`NewEnumerator9`
      (`self.PreGame`))
    (:`NewEnumerator10`
      (`self.AICinematic`))
    (:`NewEnumerator11`
      (`self.InGame`))
    (:`NewEnumerator12`
      (`self.PostGame`)))
  (`self.OnGameStateChange` _gamestate)
  (`KismetSystemLibrary.PrintString` (`|GetEnumeratorNameAsString` _gamestate)))

(fn `GetElementalGameState`
  (returns (GameState :type "/Game/Blueprints/GameMode/BP_Gamestate Object Reference"))
  (return self))

(fn `InGame`
  (`KismetSystemLibrary.PrintString` "Start AI"))

(fn `Initialization`
  (`KismetSystemLibrary.PrintString` "Initalize Game"))

(fn `PostGame`)

(fn `PreGame`
  (if (`self.HasBegunPlay`)
    (`KismetSystemLibrary.PrintString` "Pre Game: Player picks Staff")))

(fn `UserConstructionScript`)