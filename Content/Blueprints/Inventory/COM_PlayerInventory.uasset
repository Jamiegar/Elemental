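; COM_PlayerInventory is a player inventory component that holds a single weapon and swaps it when the player interacts.
; OnInteraction takes the first interacted actor, then detaches any held weapon, moves it to that actor's transform and sends it a drop message.
; It then calls InteractMessage on the actor, passing the owner, and stores the weapon obtained through GetWeaponMessage.
; GetWeaponFromInventory exposes the stored weapon.
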(fn `GetWeaponFromInventory`
  (returns (Weapon :type "/Game/Blueprints/ElementalAbilitys/BP_Weapon Object Reference"))
  (return (`self.WeaponInventory`)))

(fn `OnInteraction`
  (params (`Interacted Actors` :type "Array of Actor Object Reference"))
  (locals (interactedActorTransform :type "Transform Structure"))
  (bind _output (`|GetArrayItem` `Interacted Actors`))
  (if (`KismetArrayLibrary.Array_IsValidIndex` `Interacted Actors`)
    (set `local.interactedActorTransform` (`Actor.GetTransform` _output))
    (`/Engine/EditorBlueprintResources/StandardMacros.IsValid` (`self.WeaponInventory`)
      (:`Is Valid`
        (`Actor.K2_DetachFromActor` (`self.WeaponInventory`) "KeepRelative" "KeepRelative" "KeepRelative")
        (`Actor.K2_SetActorTransform` (`self.WeaponInventory`) (`local.interactedActorTransform`) false true)
        (message `/Game/Blueprints/Interfaces/BPI_Interactable.OnDrop` (`self.WeaponInventory`)))
      (:`Is Not Valid`
        _))
    (bind _interactable (message `/Game/Blueprints/Interfaces/BPI_Interactable.Interact` _output (`self.GetOwner`)))
    (bind _weapon (message `/Game/Blueprints/Interfaces/BPI_WeaponAbility.GetWeapon` _interactable))
    (set `self.WeaponInventory` _weapon)))