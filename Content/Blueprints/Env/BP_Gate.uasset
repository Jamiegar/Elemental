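; BP_Gate is an environment gate that slides open and shut as actors overlap its trigger references, with a sound for each direction.
; Entering OpenCollision opens it and leaving closes it, while entering CloseCollision closes it and fires the GateClosedPermanently dispatcher.
; Movement requires GateActive and uses Open and Close timelines to lerp actor location, updating Isopen on finish.
; Each opening adds the current location onto OpenLocation, overwriting that offset.
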(event `self.OpenCollision.OnActorBeginOverlap`
  (params (OverlappedActor :type "Actor Object Reference") (OtherActor :type "Actor Object Reference"))
  (if (not (`self.Isopen`))
    (`self.OpenGate`)))

(event `self.OpenCollision.OnActorEndOverlap`
  (params (OverlappedActor :type "Actor Object Reference") (OtherActor :type "Actor Object Reference"))
  (if (`self.Isopen`)
    (`self.CloseGate`)))

(event `self.CloseCollision.OnActorBeginOverlap`
  (params (OverlappedActor :type "Actor Object Reference") (OtherActor :type "Actor Object Reference"))
  (if (`self.Isopen`)
    (`self.CloseGate`)
    (`self.OnGateClosedPermanently`)))

(event `OpenGate`
  (if (`self.GateActive`)
    (bind _output_get (set `self.StartingLocation` (`self.K2_GetActorLocation`)))
    (set `self.OpenLocation` (+ _output_get (`self.OpenLocation`)))
    (`/Game/SFXData/BPFL_Sound.PlaySound` self "/Game/SFXData/DataAssets/Environmental/DA_GateOpen.DA_GateOpen" (`self.K2_GetActorLocation`))
    (bind (_direction _alpha) (`Timeline|Open` :!via `PlayFromStart`)
      (:`Update`
        (`self.K2_SetActorLocation` (`KismetMathLibrary.VLerp` (`self.StartingLocation`) (`self.OpenLocation`) _alpha) false true))
      (:`Finished`
        (set `self.Isopen` true)))))

(event `CloseGate`
  (if (`self.GateActive`)
    (`/Game/SFXData/BPFL_Sound.PlaySound` self "/Game/SFXData/DataAssets/Environmental/DA_GateClose.DA_GateClose" (`self.K2_GetActorLocation`))
    (bind (_direction _alpha) (`Timeline|Close` :!via `PlayFromStart`)
      (:`Update`
        (`self.K2_SetActorLocation` (`KismetMathLibrary.VLerp` (`self.OpenLocation`) (`self.StartingLocation`) _alpha) false true))
      (:`Finished`
        (set `self.Isopen` false)))))

(fn `UserConstructionScript`)