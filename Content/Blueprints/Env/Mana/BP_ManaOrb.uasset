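; BP_ManaOrb is a mana pickup that refills the overlapping character's mana through their weapon.
; On mesh overlap, it checks for BPI_ElementalCharacter and only proceeds if current mana is below maximum.
; It adds ManaAmount to the weapon from COM_PlayerInventory, plays the DA_ManaPickUp sound and destroys itself.
; With full mana or no valid weapon, the orb stays in place.
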(event `self.StaticMesh.OnComponentBeginOverlap`
  (params (OverlappedComponent :type "PrimitiveComponent Object Reference") (OtherActor :type "Actor Object Reference") (OtherComp :type "PrimitiveComponent Object Reference") (OtherBodyIndex :type Integer) (bFromSweep :type Boolean) (SweepResult :type "HitResult Structure (by ref)"))
  (bind _weapon (`/Game/Blueprints/Inventory/COM_PlayerInventory.GetWeaponFromInventory` (`self.GetComponentByClass` OtherActor "/Game/Blueprints/Inventory/COM_PlayerInventory.COM_PlayerInventory_C")))
  (if (`KismetSystemLibrary.DoesImplementInterface` OtherActor "/Game/Blueprints/Interfaces/BPI_ElementalCharacter.BPI_ElementalCharacter_C")
    (bind (_currentmana _maxmana) (message `/Game/Blueprints/Interfaces/BPI_ElementalCharacter.GetCharacterCurrentMana` OtherActor))
    (if (< _currentmana _maxmana)
      (`/Engine/EditorBlueprintResources/StandardMacros.IsValid` _weapon
        (:`Is Valid`
          (`/Game/Blueprints/ElementalAbilitys/BP_Weapon.AddMana` _weapon (`self.ManaAmount`))
          (`/Game/SFXData/BPFL_Sound.PlaySound` self "/Game/SFXData/DataAssets/Environmental/DA_ManaPickUp.DA_ManaPickUp" (`self.K2_GetActorLocation`))
          (`self.K2_DestroyActor`))))))

(fn `UserConstructionScript`)