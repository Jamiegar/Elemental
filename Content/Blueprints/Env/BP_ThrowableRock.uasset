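; BP_ThrowableRock is a rock projectile that can rise with a shake and damages elemental characters near its impact.
; Construction randomizes rotation and selects a rock mesh, though the random range always yields the first.
; RiseToPoint uses a timeline to lerp height by an offset while jittering X and Y.
; On hit, a sphere overlap messages BP_ElementalCharacter actors with damage; if any are found, it spawns an emitter and destroys itself.
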(event `RiseToPoint`
  (params (AddingOffset :type "Float (double-precision)"))
  (bind (_returnvalue_x _returnvalue_y) (`KismetMathLibrary.BreakVector` (`self.K2_GetActorLocation`)))
  (bind (_returnvalue_x_2 _returnvalue_y_2 _returnvalue_z) (`KismetMathLibrary.BreakVector` (`self.K2_GetActorLocation`)))
  (set `self.StartingZ` _returnvalue_z)
  (set `self.EndingZ` (+ _returnvalue_z AddingOffset))
  (bind (_direction _alpharise _shake) (`Timeline|AddOffset` :!via `PlayFromStart`)
    (:`Update`
      (bind _returnvalue (`KismetMathLibrary.Lerp` -1.2 1.2 _shake))
      (`self.K2_SetActorLocation` (+ (`KismetMathLibrary.MakeVector` _returnvalue _returnvalue) (`KismetMathLibrary.MakeVector` _returnvalue_x _returnvalue_y (`KismetMathLibrary.Lerp` (`self.StartingZ`) (`self.EndingZ`) _alpharise))) false true))))

(event `self.StaticMesh.OnComponentHit`
  (params (HitComponent :type "PrimitiveComponent Object Reference") (OtherActor :type "Actor Object Reference") (OtherComp :type "PrimitiveComponent Object Reference") (NormalImpulse :type "Vector Structure") (Hit :type "HitResult Structure (by ref)"))
  (bind (_returnvalue_location _returnvalue_rotation) (`KismetMathLibrary.BreakTransform` (`self.GetTransform`)))
  (bind (_outactors _returnvalue) (`KismetSystemLibrary.SphereOverlapActors` (`.ImpactPoint` (`GameplayStatics.BreakHitResult` Hit)) (`self.HitRadius`) (`|MakeArray` "ObjectTypeQuery3" "ObjectTypeQuery4" "ObjectTypeQuery2" :!type "EObjectTypeQuery Enum") "/Game/Blueprints/Character/BP_ElementalCharacter.BP_ElementalCharacter_C"))
  (if _returnvalue
    (for _array_element _outactors
      (message `/Game/Blueprints/Interfaces/BPI_Damageable.OnProjectileActorHit` _array_element Hit (`self.ProjectileDamage`)))
    (`GameplayStatics.SpawnEmitterAtLocation` (`self.EmitterOnHit`) _returnvalue_location _returnvalue_rotation (3.0 3.0 3.0))
    (`self.K2_DestroyActor`)))

(fn `UserConstructionScript`
  (`StaticMeshComponent.SetStaticMesh` (`self.StaticMesh`) (select `int` (`KismetMathLibrary.RandomIntegerInRange` 0) :`0` "/Game/Assets/PolygonPirates/Meshes/Environments/SM_Env_Rock_01.SM_Env_Rock_01" :`1` "/Game/Assets/PolygonPirates/Meshes/Environments/SM_Env_Rock_02.SM_Env_Rock_02" :`2` "/Game/Assets/PolygonPirates/Meshes/Environments/SM_Env_Rock_03.SM_Env_Rock_03" :!type "StaticMesh Object Reference"))
  (`SceneComponent.K2_SetWorldRotation` (`self.StaticMesh`) (`KismetMathLibrary.RandomRotator` true) false false))